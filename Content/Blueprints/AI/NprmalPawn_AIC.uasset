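; AI controller for the normal pawn that sends it along a list of waypoint actors.
; On possession it caches the pawn as an AI_Pawn reference.
; Each Tick, if it is not moving and the list is non-empty, it increments the waypoint index and calls MoveToActor on that entry.
; The index is incremented before use and never wrapped or bounds-checked.
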(event EventTick
  (params (DeltaSeconds :type Float%20%28single-precision%29))
  (bind _waypoints (Variables|Default|GetWaypoints))
  (bind _waypoint (Variables|Default|GetWaypoint))
  (Utilities|FlowControl|Sequence
    (:then_0
      (if (not (Utilities|Enum|Equal(Enum) (Class|AIController|GetMoveStatus) "Moving"))
        (if (Utilities|Array|IsValidIndex _waypoints)
          (Math|Integer|IncrementInt _waypoint
            (:%20%20
              (AI|Navigation|MovetoActor (Utilities|Array|Get(acopy) _waypoints _waypoint) 3e+01 false true))))))))

(event EventOnPossess
  (params (PossessedPawn :type Pawn%20Object%20Reference))
  (bind _asai_pawn (Utilities|Casting|CastToAI_Pawn PossessedPawn))
  (Variables|Default|SetControlledPawn _asai_pawn))

(fn ConstructionScript)