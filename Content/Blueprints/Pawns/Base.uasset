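; Base pawn Blueprint that provides a random play name and a height-based death check.
; The GetName event picks PlayName from a twenty-entry name array.
; HeightsDeath tests whether the actor's Z is at or below a fixed threshold, then edits its gameplay tag container, disables input for player zero and returns the test result.
; Nothing in this Blueprint calls the check, and BeginPlay is empty.
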(event Custom|GetName
  (Variables|Default|SetPlayName (Utilities|Array|Get(acopy) (Variables|Default|GetNameArray) (Math|Random|RandomIntegerinRange 0 19))))

(event EventBeginPlay)

(event Collision|EventActorBeginOverlap
  (params (OtherActor :type Actor%20Object%20Reference)))

(fn ConstructionScript)

(fn HeightsDeath
  (bind _returnvalue (Transformation|GetActorLocation))
  (bind _returnvalue_2 (<= (.z _returnvalue) 5e+04))
  (if _returnvalue_2
    (GameplayTags|AddGameplayTag :InOutTagContainer (Variables|Default|GetContainer) :!class /Script/GameplayTags.BlueprintGameplayTagLibrary)
    (bind _output_get (Variables|Default|SetContainerArray (GameplayTags|BreakGameplayTagContainer (Variables|Default|GetContainer))))
    (Utilities|Array|RemoveItem _output_get "")
    (Variables|Default|SetContainer (GameplayTags|MakeGameplayTagContainerfromArray (Variables|Default|GetContainerArray)))
    (Input|DisableInput (Game|GetPlayerController 0)))
  (return _returnvalue_2))