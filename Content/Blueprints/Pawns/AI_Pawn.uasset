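; AI combat character with a health bar that faces the player's pawn, colored blue when both are Team.Blue, otherwise red.
; Sighting a Base pawn, unless both are blue, turns it to aim and fire a delayed EnergyBall from a particle that grows as a charge.
; Tick also jumps at traced obstacles and destroys it on HeightsDeath.
; Point damage, including hard-landing self-damage, drives health, death tags, explosion and GameInstance kill reporting.
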(event OnSeePawn(PawnSensing)
  (params (Pawn :type Pawn%20Object%20Reference))
  (bind _particlesystem (Variables|Default|GetParticleSystem))
  (bind _particlesystem_2 (Variables|Default|GetParticleSystem))
  (bind _asbase (Utilities|Casting|CastToBase Pawn))
  (if (not (and (GameplayTags|HasTag (Variables|Default|GetContainer) "(TagName=\"Team.Blue\")") (GameplayTags|HasTag (Variables|/Game/Blueprints/Pawns/Base.Base_C|GetContainer _asbase) "(TagName=\"Team.Blue\")" true)))
    (bind _returnvalue (AI|GetAIController self))
    (Pawn|SetControlRotation _returnvalue (Math|Rotator|FindLookatRotation (Transformation|GetActorLocation) (Transformation|GetActorLocation Pawn)))
    (Utilities|FlowControl|Sequence
      (:then_0
        (Utilities|FlowControl|Gate true) ; enters at Close
      )
      (:then_1
        (Utilities|FlowControl|Delay 2.0)
        (Game|SpawnActorfromClass "/Game/Blueprints/EnergyBall_BP.EnergyBall_BP_C" (Math|Transform|MakeTransform (Transformation|GetWorldLocation _particlesystem_2) (Pawn|GetControlRotation :!class /Script/Engine.Pawn) (Transformation|GetWorldScale _particlesystem_2)) "AlwaysSpawn" self 0)
        (Transformation|SetRelativeScale3D (Variables|Default|GetParticleSystem) "0, 0, 0"))
      (:then_2
        (Components|Activation|SetActive (Variables|Default|GetParticleSystem) true true)
        (Utilities|FlowControl|Gate true) ; enters at Open
      ))))

(event EventBeginPlay
  (bind _particlesystem (Variables|Default|GetParticleSystem))
  (CallFunction|GetName)
  (bind _asbase (Utilities|Casting|CastToBase (Game|GetPlayerCharacter 0)))
  (bind _ashealth_bar (Utilities|Casting|CastToHealthBar (UserInterface|GetUserWidgetObject (Variables|Default|GetWidget1))))
  (Rendering|Components|TextRender|SetText (Variables|/Game/Widgets/HealthBar.HealthBar_C|GetTextBlock_189 _ashealth_bar) (Utilities|Text|ToText(String) (Variables|Default|GetPlayName)))
  (Appearance|SetColorandOpacity (Variables|/Game/Widgets/HealthBar.HealthBar_C|GetTextBlock_189 _ashealth_bar) (select (and (GameplayTags|HasTag (Variables|/Game/Blueprints/Pawns/Base.Base_C|GetContainer _asbase) "(TagName=\"Team.Blue\")" true) (GameplayTags|HasTag (Variables|Default|GetContainer) "(TagName=\"Team.Blue\")")) (Utilities|Struct|MakeSlateColor "(R=0.000000,G=0.671000,B=1.000000,A=1.000000)") (Utilities|Struct|MakeSlateColor "(R=1.000000,G=0.000000,B=0.000000,A=1.000000)")) :!class /Script/UMG.TextBlock)
  (Class|ProgressBar|SetFillColorandOpacity (Variables|/Game/Widgets/HealthBar.HealthBar_C|GetProgressBar_26 _ashealth_bar) (select (and (GameplayTags|HasTag (Variables|/Game/Blueprints/Pawns/Base.Base_C|GetContainer _asbase) "(TagName=\"Team.Blue\")" true) (GameplayTags|HasTag (Variables|Default|GetContainer) "(TagName=\"Team.Blue\")")) "(R=0.000000,G=0.671000,B=1.000000,A=1.000000)" "(R=1.000000,G=0.000000,B=0.000000,A=1.000000)"))
  (Components|Activation|SetActive (Variables|Default|GetParticleSystem) true true)
  (Utilities|FlowControl|Gate true) ; enters at Open
)

(event Collision|EventActorBeginOverlap
  (params (OtherActor :type Actor%20Object%20Reference)))

(event EventOnLanded
  (params (Hit :type Hit%20Result%20Structure%20%28by%20ref%29))
  (bind _charactermovement (Variables|Character|GetCharacterMovement))
  (bind _velocity (Variables|/Script/Engine.MovementComponent|GetVelocity _charactermovement))
  (bind _returnvalue (* (.z _velocity) -1.0))
  (if (>= _returnvalue 1.25e+03)
    (Game|Damage|ApplyPointDamage self (/ _returnvalue 2e+01) (Transformation|GetActorLocation) Hit 0 self "/Engine/EngineDamageTypes/DmgTypeBP_Environmental.DmgTypeBP_Environmental_C")))

(event EventTick
  (params (DeltaSeconds :type Float%20%28single-precision%29))
  (bind _returnvalue (Transformation|GetActorLocation))
  (bind _returnvalue_2 (Game|GetPlayerController 0))
  (bind _particlesystem (Variables|Default|GetParticleSystem))
  (bind _returnvalue_3 (Pawn|GetControlledPawn _returnvalue_2))
  (Utilities|FlowControl|Sequence
    (:then_0
      (Utilities|FlowControl|Gate true
        (:Exit
          (Transformation|SetRelativeScale3D _particlesystem (Math|Interpolation|VInterptoConstant (Variables|/Script/Engine.SceneComponent|GetRelativeScale3D _particlesystem) "0.040000,0.040000,0.040000" (Utilities|Time|GetWorldDeltaSeconds) 0.05)))))
    (:then_1
      (bind _returnvalue_4 (Collision|LineTraceByChannel _returnvalue (+ _returnvalue (* (Transformation|GetActorForwardVector) 1e+02)) "TraceTypeQuery1" false 0 "None"))
      (if _returnvalue_4
        (Character|Jump)
        (Utilities|FlowControl|Delay 0.2)
        (Character|StopJumping)))
    (:then_2
      (Utilities|IsValid _returnvalue_3
        (:Is%20Valid
          (Transformation|SetWorldRotation (Variables|Default|GetWidget1) (Math|Rotator|FindLookatRotation (Transformation|GetWorldLocation (Variables|Default|GetWidget1)) (Transformation|GetActorLocation _returnvalue_3)) false false))))
    (:then_3
      (bind _dead_ (CallFunction|HeightsDeath))
      (if _dead_
        (Actor|DestroyActor)))))

(event Game|Damage|EventPointDamage
  (params (Damage :type Float%20%28single-precision%29) (DamageType :type Damage%20Type%20Object%20Reference) (HitLocation :type Vector :default "0, 0, 0") (HitNormal :type Vector :default "0, 0, 0") (HitComponent :type Primitive%20Component%20Object%20Reference) (BoneName :type Name :default "None") (ShotFromDirection :type Vector :default "0, 0, 0") (InstigatedBy :type Controller%20Object%20Reference) (DamageCauser :type Actor%20Object%20Reference) (HitInfo :type Hit%20Result%20Structure%20%28by%20ref%29))
  (bind _output_get (Variables|Default|SetHealth (- (Variables|Default|GetHealth) Damage)))
  (Math|Float|CompareFloat _output_get 0.0
    (:>
      (bind _ashealth_bar (Utilities|Casting|CastToHealthBar (UserInterface|GetUserWidgetObject (Variables|Default|GetWidget1))))
      (Variables|/Game/Widgets/HealthBar.HealthBar_C|SetHealth _ashealth_bar _output_get))
    (:==
      (Variables|Default|SetHealth 0.0 :!label _label)
      (GameplayTags|AddGameplayTag (Variables|Default|GetContainer) "(TagName=\"LiveState.Death\")" :!class /Script/GameplayTags.BlueprintGameplayTagLibrary)
      (bind _output_get_2 (Variables|Default|SetContainer_Arr (GameplayTags|BreakGameplayTagContainer (Variables|Default|GetContainer))))
      (Utilities|Array|RemoveItem _output_get_2 "(TagName=\"LiveState.Alive\")")
      (Variables|Default|SetContainer (GameplayTags|MakeGameplayTagContainerfromArray (Variables|Default|GetContainer_Arr)))
      (Audio|PlaySoundatLocation "/Game/SoundEffects/Explosion.Explosion" (Transformation|GetActorLocation))
      (bind _asmy_game_instance (Utilities|Casting|CastToMyGameInstance (Game|GetGameInstance)))
      (Default|Kill _asmy_game_instance DamageCauser self)
      (Effects|SpawnEmitteratLocation "/Game/ParticleSystems/PawnExplo.PawnExplo" (Transformation|GetActorLocation))
      (Actor|DestroyActor))
    (:<
      (goto _label))))

(fn ConstructionScript)