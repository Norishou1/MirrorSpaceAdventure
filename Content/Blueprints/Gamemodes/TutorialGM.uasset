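; Tutorial game mode that runs a scripted lesson of two movement stages and a combat stage.
; BeginPlay steps a TutorialText widget through timed messages, lights MovementTrigger particles for movement, and finally shows the Vicoss end screen.
; Short Delay loops poll completion flags: MovementInput sets the movement flag, and AttackActivation sets the kill flag once no AI_Pawn actors remain.
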(event Custom|MovementInput
  (Variables|Default|SetMovementFinished true))

(event Custom|AttackActivation
  (bind _outactors (Actor|GetAllActorsOfClass "/Game/Blueprints/Pawns/AI_Pawn.AI_Pawn_C" :!label _label))
  (Math|Integer|CompareInt (Utilities|Array|Length _outactors) 0
    (:>
      (Utilities|FlowControl|Delay 0.1)
      (goto _label))
    (:==
      _)
    (:<
      _))
  (CallFunction|AttackInput))

(event Custom|AttackInput
  (Variables|Default|SetKillFinished true))

(event Custom|MovementActivation
  (params (First :type Boolean))
  (bind _outactors (Actor|GetAllActorsOfClass "/Game/Blueprints/MovementTrigger.MovementTrigger_C"))
  (for _array_element _outactors
    (if (Variables|/Game/Blueprints/MovementTrigger.MovementTrigger_C|GetFirst _array_element)
      (Variables|Default|SetFirst true)
      (Components|Activation|Activate (Variables|/Game/Blueprints/MovementTrigger.MovementTrigger_C|GetParticleSystem _array_element) true)
      (elif (not First)
        (Components|Activation|Activate (Variables|/Game/Blueprints/MovementTrigger.MovementTrigger_C|GetParticleSystem _array_element) true)))))

(event EventBeginPlay
  (bind _returnvalue (UserInterface|CreateWidget "/Game/Widgets/TutorialText.TutorialText_C" (Game|GetPlayerController 0)))
  (bind _output_get (Variables|Default|SetTextWidget _returnvalue))
  (UserInterface|Viewport|AddtoViewport _output_get 0)
  (Default|ChangeText (Variables|Default|GetTextWidget))
  (Utilities|FlowControl|Delay 5.0)
  (Default|ChangeText (Variables|Default|GetTextWidget))
  (Utilities|FlowControl|Delay 4.0)
  (Default|ChangeText (Variables|Default|GetTextWidget))
  (Utilities|FlowControl|Delay 4.0)
  (Default|ChangeText (Variables|Default|GetTextWidget))
  (Utilities|FlowControl|Delay 4.0)
  (Default|ChangeText (Variables|Default|GetTextWidget))
  (CallFunction|MovementActivation true)
  (if (Variables|Default|GetMovementFinished) :!label _label
    (Variables|Default|SetMovementFinished false)
    (Default|ChangeText (Variables|Default|GetTextWidget))
    (Utilities|FlowControl|Delay 5.0)
    (Default|ChangeText (Variables|Default|GetTextWidget))
    (Utilities|FlowControl|Delay 6.0)
    (Default|ChangeText (Variables|Default|GetTextWidget))
    (Utilities|FlowControl|Delay 5.0)
    (Default|ChangeText (Variables|Default|GetTextWidget))
    (Utilities|FlowControl|Delay 4.0)
    (Default|ChangeText (Variables|Default|GetTextWidget))
    (CallFunction|MovementActivation false)
    (if (Variables|Default|GetMovementFinished) :!label _label_2
      (Variables|Default|SetMovementFinished false)
      (Default|ChangeText (Variables|Default|GetTextWidget))
      (Utilities|FlowControl|Delay 4.0)
      (Default|ChangeText (Variables|Default|GetTextWidget))
      (Utilities|FlowControl|Delay 4.0)
      (Default|ChangeText (Variables|Default|GetTextWidget))
      (Utilities|FlowControl|Delay 4.0)
      (Default|ChangeText (Variables|Default|GetTextWidget))
      (CallFunction|AttackActivation)
      (if (Variables|Default|GetKillFinished) :!label _label_3
        (Variables|Default|SetKillFinished false)
        (Default|ChangeText (Variables|Default|GetTextWidget))
        (Utilities|FlowControl|Delay 4.0)
        (Default|ChangeText (Variables|Default|GetTextWidget))
        (Utilities|FlowControl|Delay 4.0)
        (Default|ChangeText (Variables|Default|GetTextWidget))
        (Utilities|FlowControl|Delay 4.0)
        (Default|ChangeText (Variables|Default|GetTextWidget))
        (Utilities|FlowControl|Delay 2.0)
        (Default|ChangeText (Variables|Default|GetTextWidget))
        (Utilities|FlowControl|Delay 4.0)
        (Default|ChangeText (Variables|Default|GetTextWidget))
        (Utilities|FlowControl|Delay 4.0)
        (Default|ChangeText (Variables|Default|GetTextWidget))
        (Utilities|FlowControl|Delay 2.0)
        (bind _returnvalue_2 (UserInterface|CreateWidget "/Game/Widgets/Vicoss.Vicoss_C" (Game|GetPlayerController 0)))
        (Default|StateInput _returnvalue_2 true)
        (UserInterface|Viewport|AddtoViewport _returnvalue_2 0)
        (else
          (Utilities|FlowControl|Delay 0.1)
          (goto _label_3)))
      (else
        (Utilities|FlowControl|Delay 0.1)
        (goto _label_2)))
    (else
      (Utilities|FlowControl|Delay 0.1)
      (goto _label))))

(event Collision|EventActorBeginOverlap
  (params (OtherActor :type Actor%20Object%20Reference)))

(event EventTick
  (params (DeltaSeconds :type Float%20%28single-precision%29)))

(fn ConstructionScript)