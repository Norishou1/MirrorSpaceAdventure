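; MyGameInstance is the game instance Blueprint that posts kill events to an on-screen killfeed.
; Its Kill event reads the Team.Red gameplay tag from killer and victim (Opfer) through casts to Base, treating a non-Base killer as red.
; It creates a Killbar widget for the first player controller, passes in both actors and team flags, then adds it with padding to the Killfeed scroll box.
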(event Custom|Kill
  (params (Killer :type Actor%20Object%20Reference) (Opfer :type Actor%20Object%20Reference))
  (bind _asbase (Utilities|Casting|CastToBase Killer)
    (:then
      (Variables|Default|SetKillerRed (GameplayTags|HasTag (Variables|/Game/Blueprints/Pawns/Base.Base_C|GetContainer _asbase) "(TagName=\"Team.Red\")" true)))
    (:CastFailed
      (Variables|Default|SetKillerRed true)))
  (bind _asbase_2 (Utilities|Casting|CastToBase Opfer)
    (:then
      _)
    (:CastFailed
      _))
  (bind _returnvalue (UserInterface|CreateWidget "/Game/Widgets/Killbar.Killbar_C" (Game|GetPlayerController 0)))
  (Default|Input _returnvalue Killer Opfer (GameplayTags|HasTag (Variables|/Game/Blueprints/Pawns/Base.Base_C|GetContainer _asbase_2) "(TagName=\"Team.Red\")" true) (Variables|Default|GetKillerRed))
  (bind _returnvalue_2 (Widget|Panel|AddChild (Variables|/Game/Widgets/Killfeed.Killfeed_C|GetScrollBox_99 (Variables|Default|GetKillfeed)) _returnvalue))
  (bind _asscroll_box_slot (Utilities|Casting|CastToScrollBoxSlot _returnvalue_2))
  (Layout|BorderSlot|SetPadding _asscroll_box_slot (Utilities|Struct|MakeMargin 5.0 5.0 5.0 5.0) :!class /Script/UMG.ScrollBoxSlot))