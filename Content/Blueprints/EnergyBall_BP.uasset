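; EnergyBall is an energy ball actor that deals energy point damage to what it overlaps, excluding its owner.
; The Sphere overlap skips hits where owner and target are both Base actors tagged Team.Blue; no other team is checked.
; A hit scales damage and sound volume by actor scale, activates particles, removes the ball and destroys the actor shortly after.
; A BeginPlay timer destroys it after a fixed lifetime.
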(event OnComponentBeginOverlap(Sphere)
  (params (OverlappedComponent :type Primitive%20Component%20Object%20Reference) (OtherActor :type Actor%20Object%20Reference) (OtherComp :type Primitive%20Component%20Object%20Reference) (OtherBodyIndex :type Integer) (bFromSweep :type Boolean) (SweepResult :type Hit%20Result%20Structure%20%28by%20ref%29))
  (bind _returnvalue (Components|GetOwner))
  (bind _returnvalue_2 (Transformation|GetActorScale3D))
  (bind _returnvalue_3 (/ (.x _returnvalue_2) 0.04))
  (bind _returnvalue_4 (* _returnvalue_3 5e+01))
  (Utilities|IsValid _returnvalue
    (:Is%20Valid
      (bind _asbase (Utilities|Casting|CastToBase _returnvalue))
      (bind _asbase_2 (Utilities|Casting|CastToBase OtherActor)
        (:then
          (if (not (and (GameplayTags|HasTag (Variables|/Game/Blueprints/Pawns/Base.Base_C|GetContainer _asbase) "(TagName=\"Team.Blue\")" true) (GameplayTags|HasTag (Variables|/Game/Blueprints/Pawns/Base.Base_C|GetContainer _asbase_2) "(TagName=\"Team.Blue\")" true)))
            (if (not (== OtherActor (Components|GetOwner))) :!label _label
              (Game|Damage|ApplyPointDamage OtherActor _returnvalue_4 (Transformation|GetActorLocation) SweepResult 0 (Components|GetOwner) "/Game/Blueprints/DamageTypes/DmgType_Energy.DmgType_Energy_C")
              (Components|Activation|Activate (Variables|Default|GetParticleSystem) false)
              (Components|DestroyComponent (Variables|Default|GetBall))
              (Variables|/Script/Engine.PrimitiveComponent|SetbGenerateOverlapEvents (Variables|Default|GetSphere) false)
              (Audio|PlaySoundatLocation "/Game/SoundEffects/Laser_01.Laser_01" (Transformation|GetActorLocation) "0, 0, 0" (/ _returnvalue_4 85.001))
              (Utilities|FlowControl|Delay 1.0)
              (Actor|DestroyActor))))
        (:CastFailed
          (goto _label))))
    (:Is%20Not%20Valid
      (goto _label))))

(event EventBeginPlay
  (Utilities|FlowControl|Sequence
    (:then_1
      (Utilities|FlowControl|Delay 2e+01)
      (Utilities|IsValid self
        (:Is%20Valid
          (Actor|DestroyActor))))))

(event Collision|EventActorBeginOverlap
  (params (OtherActor :type Actor%20Object%20Reference)))

(fn ConstructionScript)