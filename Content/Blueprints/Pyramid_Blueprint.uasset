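; Pyramid capture objective for a Blue vs Red team match that also inflicts environmental damage on actors standing on it.
; Nine box triggers add a stage per overlap, so overlapping more boxes speeds a team's capture and stacks the damage applied every 0.1 seconds.
; Tick advances both progress bars and ends the match on full capture or when a wiped-out team trails.
; TimeOut compares capture times; endings show the Vicoss result widget.
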(event OnComponentBeginOverlap(Box)
  (params (OverlappedComponent :type Primitive%20Component%20Object%20Reference) (OtherActor :type Actor%20Object%20Reference) (OtherComp :type Primitive%20Component%20Object%20Reference) (OtherBodyIndex :type Integer) (bFromSweep :type Boolean) (SweepResult :type Hit%20Result%20Structure%20%28by%20ref%29))
  (Variables|Default|SetotherActor OtherActor)
  (Utilities|Array|Add (Variables|Default|GetActorstocausedamage) (Variables|Default|GetotherActor))
  (bind _asbase (Utilities|Casting|CastToBase (Variables|Default|GetotherActor)))
  (if (GameplayTags|HasTag (Variables|/Game/Blueprints/Pawns/Base.Base_C|GetContainer _asbase) "(TagName=\"Team.Blue\")")
    (Utilities|Array|AddUnique (Variables|Default|GetActorsTeam1) (Variables|Default|GetotherActor))
    (Math|Integer|IncrementInt (Variables|Default|GetStagesTeam1))
    (else
      (Utilities|Array|AddUnique (Variables|Default|GetActorsTeam2) (Variables|Default|GetotherActor))
      (Math|Integer|IncrementInt (Variables|Default|GetStagesTeam2)))))

(event OnComponentBeginOverlap(Box7)
  (params (OverlappedComponent :type Primitive%20Component%20Object%20Reference) (OtherActor :type Actor%20Object%20Reference) (OtherComp :type Primitive%20Component%20Object%20Reference) (OtherBodyIndex :type Integer) (bFromSweep :type Boolean) (SweepResult :type Hit%20Result%20Structure%20%28by%20ref%29))
  (Variables|Default|SetotherActor OtherActor)
  (Utilities|Array|Add (Variables|Default|GetActorstocausedamage) (Variables|Default|GetotherActor))
  (bind _asbase (Utilities|Casting|CastToBase (Variables|Default|GetotherActor)))
  (if (GameplayTags|HasTag (Variables|/Game/Blueprints/Pawns/Base.Base_C|GetContainer _asbase) "(TagName=\"Team.Blue\")")
    (Utilities|Array|AddUnique (Variables|Default|GetActorsTeam1) (Variables|Default|GetotherActor))
    (Math|Integer|IncrementInt (Variables|Default|GetStagesTeam1))
    (else
      (Utilities|Array|AddUnique (Variables|Default|GetActorsTeam2) (Variables|Default|GetotherActor))
      (Math|Integer|IncrementInt (Variables|Default|GetStagesTeam2)))))

(event OnComponentBeginOverlap(Box6)
  (params (OverlappedComponent :type Primitive%20Component%20Object%20Reference) (OtherActor :type Actor%20Object%20Reference) (OtherComp :type Primitive%20Component%20Object%20Reference) (OtherBodyIndex :type Integer) (bFromSweep :type Boolean) (SweepResult :type Hit%20Result%20Structure%20%28by%20ref%29))
  (Variables|Default|SetotherActor OtherActor)
  (Utilities|Array|Add (Variables|Default|GetActorstocausedamage) (Variables|Default|GetotherActor))
  (bind _asbase (Utilities|Casting|CastToBase (Variables|Default|GetotherActor)))
  (if (GameplayTags|HasTag (Variables|/Game/Blueprints/Pawns/Base.Base_C|GetContainer _asbase) "(TagName=\"Team.Blue\")")
    (Utilities|Array|AddUnique (Variables|Default|GetActorsTeam1) (Variables|Default|GetotherActor))
    (Math|Integer|IncrementInt (Variables|Default|GetStagesTeam1))
    (else
      (Utilities|Array|AddUnique (Variables|Default|GetActorsTeam2) (Variables|Default|GetotherActor))
      (Math|Integer|IncrementInt (Variables|Default|GetStagesTeam2)))))

(event OnComponentBeginOverlap(Box5)
  (params (OverlappedComponent :type Primitive%20Component%20Object%20Reference) (OtherActor :type Actor%20Object%20Reference) (OtherComp :type Primitive%20Component%20Object%20Reference) (OtherBodyIndex :type Integer) (bFromSweep :type Boolean) (SweepResult :type Hit%20Result%20Structure%20%28by%20ref%29))
  (Variables|Default|SetotherActor OtherActor)
  (Utilities|Array|Add (Variables|Default|GetActorstocausedamage) (Variables|Default|GetotherActor))
  (bind _asbase (Utilities|Casting|CastToBase (Variables|Default|GetotherActor)))
  (if (GameplayTags|HasTag (Variables|/Game/Blueprints/Pawns/Base.Base_C|GetContainer _asbase) "(TagName=\"Team.Blue\")")
    (Utilities|Array|AddUnique (Variables|Default|GetActorsTeam1) (Variables|Default|GetotherActor))
    (Math|Integer|IncrementInt (Variables|Default|GetStagesTeam1))
    (else
      (Utilities|Array|AddUnique (Variables|Default|GetActorsTeam2) (Variables|Default|GetotherActor))
      (Math|Integer|IncrementInt (Variables|Default|GetStagesTeam2)))))

(event OnComponentBeginOverlap(Box4)
  (params (OverlappedComponent :type Primitive%20Component%20Object%20Reference) (OtherActor :type Actor%20Object%20Reference) (OtherComp :type Primitive%20Component%20Object%20Reference) (OtherBodyIndex :type Integer) (bFromSweep :type Boolean) (SweepResult :type Hit%20Result%20Structure%20%28by%20ref%29))
  (Variables|Default|SetotherActor OtherActor)
  (Utilities|Array|Add (Variables|Default|GetActorstocausedamage) (Variables|Default|GetotherActor))
  (bind _asbase (Utilities|Casting|CastToBase (Variables|Default|GetotherActor)))
  (if (GameplayTags|HasTag (Variables|/Game/Blueprints/Pawns/Base.Base_C|GetContainer _asbase) "(TagName=\"Team.Blue\")")
    (Utilities|Array|AddUnique (Variables|Default|GetActorsTeam1) (Variables|Default|GetotherActor))
    (Math|Integer|IncrementInt (Variables|Default|GetStagesTeam1))
    (else
      (Utilities|Array|AddUnique (Variables|Default|GetActorsTeam2) (Variables|Default|GetotherActor))
      (Math|Integer|IncrementInt (Variables|Default|GetStagesTeam2)))))

(event OnComponentBeginOverlap(Box3)
  (params (OverlappedComponent :type Primitive%20Component%20Object%20Reference) (OtherActor :type Actor%20Object%20Reference) (OtherComp :type Primitive%20Component%20Object%20Reference) (OtherBodyIndex :type Integer) (bFromSweep :type Boolean) (SweepResult :type Hit%20Result%20Structure%20%28by%20ref%29))
  (Variables|Default|SetotherActor OtherActor)
  (Utilities|Array|Add (Variables|Default|GetActorstocausedamage) (Variables|Default|GetotherActor))
  (bind _asbase (Utilities|Casting|CastToBase (Variables|Default|GetotherActor)))
  (if (GameplayTags|HasTag (Variables|/Game/Blueprints/Pawns/Base.Base_C|GetContainer _asbase) "(TagName=\"Team.Blue\")")
    (Utilities|Array|AddUnique (Variables|Default|GetActorsTeam1) (Variables|Default|GetotherActor))
    (Math|Integer|IncrementInt (Variables|Default|GetStagesTeam1))
    (else
      (Utilities|Array|AddUnique (Variables|Default|GetActorsTeam2) (Variables|Default|GetotherActor))
      (Math|Integer|IncrementInt (Variables|Default|GetStagesTeam2)))))

(event OnComponentBeginOverlap(Box2)
  (params (OverlappedComponent :type Primitive%20Component%20Object%20Reference) (OtherActor :type Actor%20Object%20Reference) (OtherComp :type Primitive%20Component%20Object%20Reference) (OtherBodyIndex :type Integer) (bFromSweep :type Boolean) (SweepResult :type Hit%20Result%20Structure%20%28by%20ref%29))
  (Variables|Default|SetotherActor OtherActor)
  (Utilities|Array|Add (Variables|Default|GetActorstocausedamage) (Variables|Default|GetotherActor))
  (bind _asbase (Utilities|Casting|CastToBase (Variables|Default|GetotherActor)))
  (if (GameplayTags|HasTag (Variables|/Game/Blueprints/Pawns/Base.Base_C|GetContainer _asbase) "(TagName=\"Team.Blue\")")
    (Utilities|Array|AddUnique (Variables|Default|GetActorsTeam1) (Variables|Default|GetotherActor))
    (Math|Integer|IncrementInt (Variables|Default|GetStagesTeam1))
    (else
      (Utilities|Array|AddUnique (Variables|Default|GetActorsTeam2) (Variables|Default|GetotherActor))
      (Math|Integer|IncrementInt (Variables|Default|GetStagesTeam2)))))

(event OnComponentBeginOverlap(Box1)
  (params (OverlappedComponent :type Primitive%20Component%20Object%20Reference) (OtherActor :type Actor%20Object%20Reference) (OtherComp :type Primitive%20Component%20Object%20Reference) (OtherBodyIndex :type Integer) (bFromSweep :type Boolean) (SweepResult :type Hit%20Result%20Structure%20%28by%20ref%29))
  (Variables|Default|SetotherActor OtherActor)
  (Utilities|Array|Add (Variables|Default|GetActorstocausedamage) (Variables|Default|GetotherActor))
  (bind _asbase (Utilities|Casting|CastToBase (Variables|Default|GetotherActor)))
  (if (GameplayTags|HasTag (Variables|/Game/Blueprints/Pawns/Base.Base_C|GetContainer _asbase) "(TagName=\"Team.Blue\")")
    (Utilities|Array|AddUnique (Variables|Default|GetActorsTeam1) (Variables|Default|GetotherActor))
    (Math|Integer|IncrementInt (Variables|Default|GetStagesTeam1))
    (else
      (Utilities|Array|AddUnique (Variables|Default|GetActorsTeam2) (Variables|Default|GetotherActor))
      (Math|Integer|IncrementInt (Variables|Default|GetStagesTeam2)))))

(event OnComponentEndOverlap(Box8)
  (params (OverlappedComponent :type Primitive%20Component%20Object%20Reference) (OtherActor :type Actor%20Object%20Reference) (OtherComp :type Primitive%20Component%20Object%20Reference) (OtherBodyIndex :type Integer))
  (bind _actorstocausedamage (Variables|Default|GetActorstocausedamage))
  (Variables|Default|SetotherActor OtherActor)
  (bind (_array_element _array_index) (Utilities|Array|ForEachLoopwithBreak _actorstocausedamage :!label _label)
    (:LoopBody
      (if (== (Variables|Default|GetotherActor) _array_element)
        (Utilities|Array|RemoveIndex _actorstocausedamage _array_index)
        (goto _label Break)))
    (:Completed
      (bind _asbase (Utilities|Casting|CastToBase (Variables|Default|GetotherActor)))
      (if (GameplayTags|HasTag (Variables|/Game/Blueprints/Pawns/Base.Base_C|GetContainer _asbase) "(TagName=\"Team.Blue\")" true)
        (Utilities|Array|RemoveItem (Variables|Default|GetActorsTeam1) (Variables|Default|GetotherActor))
        (Math|Integer|DecrementInt (Variables|Default|GetStagesTeam1))
        (else
          (Utilities|Array|RemoveItem (Variables|Default|GetActorsTeam2) (Variables|Default|GetotherActor))
          (Math|Integer|DecrementInt (Variables|Default|GetStagesTeam2)))))))

(event OnComponentEndOverlap(Box7)
  (params (OverlappedComponent :type Primitive%20Component%20Object%20Reference) (OtherActor :type Actor%20Object%20Reference) (OtherComp :type Primitive%20Component%20Object%20Reference) (OtherBodyIndex :type Integer))
  (bind _actorstocausedamage (Variables|Default|GetActorstocausedamage))
  (Variables|Default|SetotherActor OtherActor)
  (bind (_array_element _array_index) (Utilities|Array|ForEachLoopwithBreak _actorstocausedamage :!label _label)
    (:LoopBody
      (if (== (Variables|Default|GetotherActor) _array_element)
        (Utilities|Array|RemoveIndex _actorstocausedamage _array_index)
        (goto _label Break)))
    (:Completed
      (bind _asbase (Utilities|Casting|CastToBase (Variables|Default|GetotherActor)))
      (if (GameplayTags|HasTag (Variables|/Game/Blueprints/Pawns/Base.Base_C|GetContainer _asbase) "(TagName=\"Team.Blue\")" true)
        (Utilities|Array|RemoveItem (Variables|Default|GetActorsTeam1) (Variables|Default|GetotherActor))
        (Math|Integer|DecrementInt (Variables|Default|GetStagesTeam1))
        (else
          (Utilities|Array|RemoveItem (Variables|Default|GetActorsTeam2) (Variables|Default|GetotherActor))
          (Math|Integer|DecrementInt (Variables|Default|GetStagesTeam2)))))))

(event OnComponentEndOverlap(Box6)
  (params (OverlappedComponent :type Primitive%20Component%20Object%20Reference) (OtherActor :type Actor%20Object%20Reference) (OtherComp :type Primitive%20Component%20Object%20Reference) (OtherBodyIndex :type Integer))
  (bind _actorstocausedamage (Variables|Default|GetActorstocausedamage))
  (Variables|Default|SetotherActor OtherActor)
  (bind (_array_element _array_index) (Utilities|Array|ForEachLoopwithBreak _actorstocausedamage :!label _label)
    (:LoopBody
      (if (== (Variables|Default|GetotherActor) _array_element)
        (Utilities|Array|RemoveIndex _actorstocausedamage _array_index)
        (goto _label Break)))
    (:Completed
      (bind _asbase (Utilities|Casting|CastToBase (Variables|Default|GetotherActor)))
      (if (GameplayTags|HasTag (Variables|/Game/Blueprints/Pawns/Base.Base_C|GetContainer _asbase) "(TagName=\"Team.Blue\")" true)
        (Utilities|Array|RemoveItem (Variables|Default|GetActorsTeam1) (Variables|Default|GetotherActor))
        (Math|Integer|DecrementInt (Variables|Default|GetStagesTeam1))
        (else
          (Utilities|Array|RemoveItem (Variables|Default|GetActorsTeam2) (Variables|Default|GetotherActor))
          (Math|Integer|DecrementInt (Variables|Default|GetStagesTeam2)))))))

(event OnComponentEndOverlap(Box5)
  (params (OverlappedComponent :type Primitive%20Component%20Object%20Reference) (OtherActor :type Actor%20Object%20Reference) (OtherComp :type Primitive%20Component%20Object%20Reference) (OtherBodyIndex :type Integer))
  (bind _actorstocausedamage (Variables|Default|GetActorstocausedamage))
  (Variables|Default|SetotherActor OtherActor)
  (bind (_array_element _array_index) (Utilities|Array|ForEachLoopwithBreak _actorstocausedamage :!label _label)
    (:LoopBody
      (if (== (Variables|Default|GetotherActor) _array_element)
        (Utilities|Array|RemoveIndex _actorstocausedamage _array_index)
        (goto _label Break)))
    (:Completed
      (bind _asbase (Utilities|Casting|CastToBase (Variables|Default|GetotherActor)))
      (if (GameplayTags|HasTag (Variables|/Game/Blueprints/Pawns/Base.Base_C|GetContainer _asbase) "(TagName=\"Team.Blue\")" true)
        (Utilities|Array|RemoveItem (Variables|Default|GetActorsTeam1) (Variables|Default|GetotherActor))
        (Math|Integer|DecrementInt (Variables|Default|GetStagesTeam1))
        (else
          (Utilities|Array|RemoveItem (Variables|Default|GetActorsTeam2) (Variables|Default|GetotherActor))
          (Math|Integer|DecrementInt (Variables|Default|GetStagesTeam2)))))))

(event OnComponentEndOverlap(Box4)
  (params (OverlappedComponent :type Primitive%20Component%20Object%20Reference) (OtherActor :type Actor%20Object%20Reference) (OtherComp :type Primitive%20Component%20Object%20Reference) (OtherBodyIndex :type Integer))
  (bind _actorstocausedamage (Variables|Default|GetActorstocausedamage))
  (Variables|Default|SetotherActor OtherActor)
  (bind (_array_element _array_index) (Utilities|Array|ForEachLoopwithBreak _actorstocausedamage :!label _label)
    (:LoopBody
      (if (== (Variables|Default|GetotherActor) _array_element)
        (Utilities|Array|RemoveIndex _actorstocausedamage _array_index)
        (goto _label Break)))
    (:Completed
      (bind _asbase (Utilities|Casting|CastToBase (Variables|Default|GetotherActor)))
      (if (GameplayTags|HasTag (Variables|/Game/Blueprints/Pawns/Base.Base_C|GetContainer _asbase) "(TagName=\"Team.Blue\")" true)
        (Utilities|Array|RemoveItem (Variables|Default|GetActorsTeam1) (Variables|Default|GetotherActor))
        (Math|Integer|DecrementInt (Variables|Default|GetStagesTeam1))
        (else
          (Utilities|Array|RemoveItem (Variables|Default|GetActorsTeam2) (Variables|Default|GetotherActor))
          (Math|Integer|DecrementInt (Variables|Default|GetStagesTeam2)))))))

(event OnComponentEndOverlap(Box3)
  (params (OverlappedComponent :type Primitive%20Component%20Object%20Reference) (OtherActor :type Actor%20Object%20Reference) (OtherComp :type Primitive%20Component%20Object%20Reference) (OtherBodyIndex :type Integer))
  (bind _actorstocausedamage (Variables|Default|GetActorstocausedamage))
  (Variables|Default|SetotherActor OtherActor)
  (bind (_array_element _array_index) (Utilities|Array|ForEachLoopwithBreak _actorstocausedamage :!label _label)
    (:LoopBody
      (if (== (Variables|Default|GetotherActor) _array_element)
        (Utilities|Array|RemoveIndex _actorstocausedamage _array_index)
        (goto _label Break)))
    (:Completed
      (bind _asbase (Utilities|Casting|CastToBase (Variables|Default|GetotherActor)))
      (if (GameplayTags|HasTag (Variables|/Game/Blueprints/Pawns/Base.Base_C|GetContainer _asbase) "(TagName=\"Team.Blue\")" true)
        (Utilities|Array|RemoveItem (Variables|Default|GetActorsTeam1) (Variables|Default|GetotherActor))
        (Math|Integer|DecrementInt (Variables|Default|GetStagesTeam1))
        (else
          (Utilities|Array|RemoveItem (Variables|Default|GetActorsTeam2) (Variables|Default|GetotherActor))
          (Math|Integer|DecrementInt (Variables|Default|GetStagesTeam2)))))))

(event OnComponentEndOverlap(Box2)
  (params (OverlappedComponent :type Primitive%20Component%20Object%20Reference) (OtherActor :type Actor%20Object%20Reference) (OtherComp :type Primitive%20Component%20Object%20Reference) (OtherBodyIndex :type Integer))
  (bind _actorstocausedamage (Variables|Default|GetActorstocausedamage))
  (Variables|Default|SetotherActor OtherActor)
  (bind (_array_element _array_index) (Utilities|Array|ForEachLoopwithBreak _actorstocausedamage :!label _label)
    (:LoopBody
      (if (== (Variables|Default|GetotherActor) _array_element)
        (Utilities|Array|RemoveIndex _actorstocausedamage _array_index)
        (goto _label Break)))
    (:Completed
      (bind _asbase (Utilities|Casting|CastToBase (Variables|Default|GetotherActor)))
      (if (GameplayTags|HasTag (Variables|/Game/Blueprints/Pawns/Base.Base_C|GetContainer _asbase) "(TagName=\"Team.Blue\")" true)
        (Utilities|Array|RemoveItem (Variables|Default|GetActorsTeam1) (Variables|Default|GetotherActor))
        (Math|Integer|DecrementInt (Variables|Default|GetStagesTeam1))
        (else
          (Utilities|Array|RemoveItem (Variables|Default|GetActorsTeam2) (Variables|Default|GetotherActor))
          (Math|Integer|DecrementInt (Variables|Default|GetStagesTeam2)))))))

(event OnComponentEndOverlap(Box1)
  (params (OverlappedComponent :type Primitive%20Component%20Object%20Reference) (OtherActor :type Actor%20Object%20Reference) (OtherComp :type Primitive%20Component%20Object%20Reference) (OtherBodyIndex :type Integer))
  (bind _actorstocausedamage (Variables|Default|GetActorstocausedamage))
  (Variables|Default|SetotherActor OtherActor)
  (bind (_array_element _array_index) (Utilities|Array|ForEachLoopwithBreak _actorstocausedamage :!label _label)
    (:LoopBody
      (if (== (Variables|Default|GetotherActor) _array_element)
        (Utilities|Array|RemoveIndex _actorstocausedamage _array_index)
        (goto _label Break)))
    (:Completed
      (bind _asbase (Utilities|Casting|CastToBase (Variables|Default|GetotherActor)))
      (if (GameplayTags|HasTag (Variables|/Game/Blueprints/Pawns/Base.Base_C|GetContainer _asbase) "(TagName=\"Team.Blue\")" true)
        (Utilities|Array|RemoveItem (Variables|Default|GetActorsTeam1) (Variables|Default|GetotherActor))
        (Math|Integer|DecrementInt (Variables|Default|GetStagesTeam1))
        (else
          (Utilities|Array|RemoveItem (Variables|Default|GetActorsTeam2) (Variables|Default|GetotherActor))
          (Math|Integer|DecrementInt (Variables|Default|GetStagesTeam2)))))))

(event OnComponentEndOverlap(Box)
  (params (OverlappedComponent :type Primitive%20Component%20Object%20Reference) (OtherActor :type Actor%20Object%20Reference) (OtherComp :type Primitive%20Component%20Object%20Reference) (OtherBodyIndex :type Integer))
  (bind _actorstocausedamage (Variables|Default|GetActorstocausedamage))
  (Variables|Default|SetotherActor OtherActor)
  (bind (_array_element _array_index) (Utilities|Array|ForEachLoopwithBreak _actorstocausedamage :!label _label)
    (:LoopBody
      (if (== (Variables|Default|GetotherActor) _array_element)
        (Utilities|Array|RemoveIndex _actorstocausedamage _array_index)
        (goto _label Break)))
    (:Completed
      (bind _asbase (Utilities|Casting|CastToBase (Variables|Default|GetotherActor)))
      (if (GameplayTags|HasTag (Variables|/Game/Blueprints/Pawns/Base.Base_C|GetContainer _asbase) "(TagName=\"Team.Blue\")" true)
        (Utilities|Array|RemoveItem (Variables|Default|GetActorsTeam1) (Variables|Default|GetotherActor))
        (Math|Integer|DecrementInt (Variables|Default|GetStagesTeam1))
        (else
          (Utilities|Array|RemoveItem (Variables|Default|GetActorsTeam2) (Variables|Default|GetotherActor))
          (Math|Integer|DecrementInt (Variables|Default|GetStagesTeam2)))))))

(event OnComponentBeginOverlap(Box8)
  (params (OverlappedComponent :type Primitive%20Component%20Object%20Reference) (OtherActor :type Actor%20Object%20Reference) (OtherComp :type Primitive%20Component%20Object%20Reference) (OtherBodyIndex :type Integer) (bFromSweep :type Boolean) (SweepResult :type Hit%20Result%20Structure%20%28by%20ref%29))
  (Variables|Default|SetotherActor OtherActor)
  (Utilities|Array|Add (Variables|Default|GetActorstocausedamage) (Variables|Default|GetotherActor))
  (bind _asbase (Utilities|Casting|CastToBase (Variables|Default|GetotherActor)))
  (if (GameplayTags|HasTag (Variables|/Game/Blueprints/Pawns/Base.Base_C|GetContainer _asbase) "(TagName=\"Team.Blue\")")
    (Utilities|Array|AddUnique (Variables|Default|GetActorsTeam1) (Variables|Default|GetotherActor))
    (Math|Integer|IncrementInt (Variables|Default|GetStagesTeam1))
    (else
      (Utilities|Array|AddUnique (Variables|Default|GetActorsTeam2) (Variables|Default|GetotherActor))
      (Math|Integer|IncrementInt (Variables|Default|GetStagesTeam2)))))

(event Custom|Damage
  (bind _actorstocausedamage (Variables|Default|GetActorstocausedamage))
  (for _array_element _actorstocausedamage
    (bind _asbase (Utilities|Casting|CastToBase _array_element)
      (:then
        (if (GameplayTags|HasTag (Variables|/Game/Blueprints/Pawns/Base.Base_C|GetContainer _asbase) "(TagName=\"LiveState.Death\")" true)
          (Utilities|Array|RemoveItem _actorstocausedamage _array_element)
          (else
            (Game|Damage|ApplyPointDamage _array_element (Variables|Default|GetDamageper0.1sec) (Transformation|GetActorLocation) (Collision|MakeHitResult false false 0.0 "0, 0, 0" "0, 0, 0" "0,0,1" "0,0,1" 0 0 0) 0 self "/Engine/EngineDamageTypes/DmgTypeBP_Environmental.DmgTypeBP_Environmental_C" :!label _label))))
      (:CastFailed
        (goto _label)))))

(event Custom|TimeOut
  (if (< (Variables|Default|GetTime1) (Variables|Default|GetTime2))
    (Variables|Default|SetIsActive false)
    (bind _asmy_game_instance (Utilities|Casting|CastToMyGameInstance (Game|GetGameInstance)))
    (Widget|RemovefromParent (Variables|/Game/Blueprints/MyGameInstance.MyGameInstance_C|GetCaptureState _asmy_game_instance))
    (bind _returnvalue (UserInterface|CreateWidget "/Game/Widgets/Vicoss.Vicoss_C"))
    (UserInterface|Viewport|AddtoViewport _returnvalue 0)
    (Default|StateInput _returnvalue (== (Variables|Default|GetPlayerTag) "(TagName=\"Team.Red\")"))
    (else
      (Variables|Default|SetIsActive false)
      (bind _asmy_game_instance_2 (Utilities|Casting|CastToMyGameInstance (Game|GetGameInstance)))
      (Widget|RemovefromParent (Variables|/Game/Blueprints/MyGameInstance.MyGameInstance_C|GetCaptureState _asmy_game_instance_2))
      (bind _returnvalue_2 (UserInterface|CreateWidget "/Game/Widgets/Vicoss.Vicoss_C" (Game|GetPlayerController 0)))
      (UserInterface|Viewport|AddtoViewport _returnvalue_2 0)
      (Default|StateInput _returnvalue_2 (== (Variables|Default|GetPlayerTag) "(TagName=\"Team.Blue\")")))))

(event EventBeginPlay
  (Utilities|FlowControl|Sequence
    (:then_0
      (Utilities|FlowControl|Delay 0.2)
      (bind _asbase (Utilities|Casting|CastToBase (Game|GetPlayerCharacter 0)))
      (Variables|Default|SetPlayerTag (select (GameplayTags|HasTag (Variables|/Game/Blueprints/Pawns/Base.Base_C|GetContainer _asbase) "(TagName=\"Team.Red\")" true) "(TagName=\"Team.Red\")" "(TagName=\"Team.Blue\")")))
    (:then_1
      (Utilities|FlowControl|Delay 0.1 :!label _label)
      (CallFunction|Damage)
      (if (Variables|Default|GetIsActive)
        (goto _label)))))

(event Collision|EventActorBeginOverlap
  (params (OtherActor :type Actor%20Object%20Reference)))

(event EventTick
  (params (DeltaSeconds :type Float%20%28single-precision%29))
  (if (Variables|Default|GetIsActive)
    (bind _outactors (Actor|GetAllActorsOfClass "/Game/Blueprints/Pawns/Base.Base_C"))
    (if (== (Utilities|Array|Length _outactors) 0)
      (if (< (Variables|Default|GetTime1) (Variables|Default|GetTime2))
        (Variables|Default|SetIsActive false :!label _label)
        (bind _asmy_game_instance (Utilities|Casting|CastToMyGameInstance (Game|GetGameInstance)))
        (Widget|RemovefromParent (Variables|/Game/Blueprints/MyGameInstance.MyGameInstance_C|GetCaptureState _asmy_game_instance))
        (bind _returnvalue (UserInterface|CreateWidget "/Game/Widgets/Vicoss.Vicoss_C"))
        (UserInterface|Viewport|AddtoViewport _returnvalue 0)
        (Default|StateInput _returnvalue (== (Variables|Default|GetPlayerTag) "(TagName=\"Team.Red\")"))
        (else
          (Variables|Default|SetIsActive false :!label _label_2)
          (bind _asmy_game_instance_2 (Utilities|Casting|CastToMyGameInstance (Game|GetGameInstance)))
          (Widget|RemovefromParent (Variables|/Game/Blueprints/MyGameInstance.MyGameInstance_C|GetCaptureState _asmy_game_instance_2))
          (bind _returnvalue_2 (UserInterface|CreateWidget "/Game/Widgets/Vicoss.Vicoss_C" (Game|GetPlayerController 0)))
          (UserInterface|Viewport|AddtoViewport _returnvalue_2 0)
          (Default|StateInput _returnvalue_2 (== (Variables|Default|GetPlayerTag) "(TagName=\"Team.Blue\")"))))
      (else
        (Variables|Default|SetBlueAlife false)
        (Variables|Default|SetRedAlife false)
        (for _array_element _outactors
          (if (GameplayTags|HasTag (Variables|/Game/Blueprints/Pawns/Base.Base_C|GetContainer _array_element) "(TagName=\"Team.Blue\")" true)
            (Variables|Default|SetBlueAlife true)
            (else
              (Variables|Default|SetRedAlife true))))
        (Utilities|FlowControl|Sequence
          (:then_0
            (if (Variables|Default|GetBlueAlife)
              _
              (elif (< (Variables|Default|GetTime1) (Variables|Default|GetTime2))
                (goto _label)
                (else
                  _)))
            (bind _output_get (Variables|Default|SetTime1 (+ (* (Variables|Default|GetStagesTeam1) DeltaSeconds) (Variables|Default|GetTime1))))
            (bind _output_get_2 (Variables|Default|SetProcent_Filled1 (/ _output_get (Variables|Default|GetCapture_Time))))
            (Math|Float|CompareFloat _output_get_2 1.0
              (:>
                (Variables|Default|SetProcent_Filled1 1.0)
                (goto _label_2))
              (:==
                _)
              (:<
                _))
            (bind _asmy_game_instance_3 (Utilities|Casting|CastToMyGameInstance (Game|GetGameInstance)))
            (Default|ProgressBar1 (Variables|/Game/Blueprints/MyGameInstance.MyGameInstance_C|GetCaptureState _asmy_game_instance_3) (Variables|Default|GetProcent_Filled1) (Variables|Default|GetStagesTeam1)))
          (:then_1
            (if (Variables|Default|GetRedAlife)
              _
              (elif (< (Variables|Default|GetTime2) (Variables|Default|GetTime1))
                (goto _label_2)
                (else
                  _)))
            (bind _output_get_3 (Variables|Default|SetTime2 (+ (* (Variables|Default|GetStagesTeam2) DeltaSeconds) (Variables|Default|GetTime2))))
            (bind _output_get_4 (Variables|Default|SetProcent_Filled2 (/ _output_get_3 (Variables|Default|GetCapture_Time))))
            (Math|Float|CompareFloat _output_get_4 1.0
              (:>
                (Variables|Default|SetProcent_Filled2 1.0)
                (goto _label))
              (:==
                _)
              (:<
                _))
            (bind _asmy_game_instance_4 (Utilities|Casting|CastToMyGameInstance (Game|GetGameInstance)))
            (Default|ProgressBar2 (Variables|/Game/Blueprints/MyGameInstance.MyGameInstance_C|GetCaptureState _asmy_game_instance_4) (Variables|Default|GetProcent_Filled2) (Variables|Default|GetStagesTeam2))))))))

(fn ConstructionScript)